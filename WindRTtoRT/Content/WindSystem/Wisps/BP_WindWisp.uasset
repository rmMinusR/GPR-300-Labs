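; BP_WindWisp is a short-lived wind wisp visual effect actor that animates once and then destroys itself.
; The construction script picks one of four wisp meshes at random.
; BeginPlay creates a dynamic material instance with its Sweep parameter at zero.
; Tick raises Sweep at a rate set by TimeToDestroy and destroys the actor once the value passes one, so the material parameter doubles as the lifetime timer.
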(event EventBeginPlay
  (bind _returnvalue (Rendering|Material|CreateDynamicMaterialInstance (Rendering|Material|GetMaterial (Variables|Default|GetStaticMesh) 0) "None" "None" :!class /Script/Engine.KismetMaterialLibrary))
  (Rendering|Material|SetMaterial (Variables|Default|GetStaticMesh) 0 _returnvalue)
  (Rendering|Material|SetScalarParameterValue _returnvalue "Sweep" 0.0 :!class /Script/Engine.MaterialInstanceDynamic))

(event EventTick
  (params (DeltaSeconds :type Float%20%28single-precision%29))
  (bind _returnvalue (Rendering|Material|GetScalarParameterValue (stale EventBeginPlay _returnvalue) "Sweep" :!class /Script/Engine.MaterialInstanceDynamic))
  (Rendering|Material|SetScalarParameterValue (stale EventBeginPlay _returnvalue) "Sweep" (+ _returnvalue (/ DeltaSeconds (Variables|Default|GetTime%20To%20Destroy))) :!class /Script/Engine.MaterialInstanceDynamic)
  (if (> (+ _returnvalue (/ DeltaSeconds (Variables|Default|GetTime%20To%20Destroy))) 1.0)
    (Actor|DestroyActor)))

(fn ConstructionScript
  (Components|StaticMesh|SetStaticMesh (Variables|Default|GetStaticMesh) (.OutItem (Utilities|Array|Random (Utilities|Array|MakeArray "/Game/WindSystem/Wisps/windwisp1.windwisp1" "/Game/WindSystem/Wisps/windwisp2.windwisp2" "/Game/WindSystem/Wisps/windwisp3.windwisp3" "/Game/WindSystem/Wisps/windwisp4.windwisp4")))))