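; BP_SnowCarver is an actor that leaves a trail of static mesh components as it moves, apparently to carve snow.
; Each Tick, once its root is beyond PlacementOffset from LastPlacePos, it moves that point to PlacementOffset behind the root.
; It adds an unattached mesh there, then rescales the owning actor by a bounds ratio that compares the actor with itself.
; SphereCollider's location is read but unused.
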(event EventTick
  (params (DeltaSeconds :type Float%20%28single-precision%29))
  (bind _defaultsceneroot (Variables|Default|GetDefaultSceneRoot))
  (bind _returnvalue (Transformation|GetWorldLocation _defaultsceneroot))
  (if (> (Math|Vector|VectorLength (- (Variables|Default|GetLastPlacePos) _returnvalue)) (Variables|Default|GetPlacementOffset))
    (Variables|Default|SetLastPlacePos (+ (* (Math|Vector|Normalize (- (Variables|Default|GetLastPlacePos) _returnvalue)) (Variables|Default|GetPlacementOffset)) _returnvalue))
    (bind _returnvalue_2 (AddComponent|AddStaticMeshComponent true (Math|Conversions|ToTransform(Vector) (+ (* (Math|Vector|Normalize (- (Variables|Default|GetLastPlacePos) _returnvalue)) (Variables|Default|GetPlacementOffset)) _returnvalue))))
    (Transformation|SetActorScale3D (Components|GetOwner _returnvalue_2) (/ (.BoxExtent (Collision|GetActorBounds (Components|GetOwner _returnvalue_2) false false)) (.BoxExtent (Collision|GetActorBounds false false))))))

(fn ConstructionScript)